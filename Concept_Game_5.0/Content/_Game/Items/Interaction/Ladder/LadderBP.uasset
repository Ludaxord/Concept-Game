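; LadderBP is a ladder interaction actor with a pickup widget, built procedurally in its construction script.
; The construction script runs setup functions in sequence for mesh size, rungs, area capsule, climb box collision, and upper, bottom and disable-collision capsules.
; On BeginPlay it passes itself to the ItemInteractionWidgetBP as the item reference.
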(event `self.ReceiveBeginPlay`
  (bind _asitem_interaction_widget_bp (cast `/Game/_Game/HUD/Widgets/Items/ItemInteractionWidgetBP` (`WidgetComponent.GetUserWidgetObject` (`self.PickupWidget`))))
  (set `/Game/_Game/HUD/Widgets/Items/ItemInteractionWidgetBP.ItemReference` self _asitem_interaction_widget_bp))

(fn `UserConstructionScript`
  (`|ExecutionSequence`
    (:`then_0`
      (`self.SetupLadderMeshSize`))
    (:`then_1`
      (`self.SetupAreaCapsule`))
    (:`then_2`
      (`self.SetupLadderRungs`))
    (:`then_3`
      (`self.SetupClimbLadderBoxCollision`))
    (:`then_4`
      (`self.SetupUpperCapsule`))
    (:`then_5`
      (`self.SetupBottomCapsule`))
    (:`then_6`
      (`self.SetupDisableCollisionCapsule`))))