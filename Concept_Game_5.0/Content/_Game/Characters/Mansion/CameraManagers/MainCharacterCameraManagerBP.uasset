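; Player camera manager for MainCharacter that handles first-person aim-down-sights with an equipped weapon.
; BlueprintUpdateCamera overrides the view only while EyesCamera is active and a weapon is valid, keeping control rotation.
; CurrentAimValue blends location from the eyes toward a point on the weapon's Ironsight socket axis, computed from the eye-to-sight vector, and narrows FOV.
; SwayOffset, rotated into view space, is added to the final location.
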(fn `BlueprintUpdateCamera`
  (params (CameraTarget :type "Actor Object Reference"))
  (returns (NewCameraLocation :type "Vector Structure") (NewCameraRotation :type "Rotator Structure") (NewCameraFOV :type "Float (single-precision)") (ReturnValue :type Boolean))
  (bind _equippedweapon (`MainCharacter.EquippedWeapon` (`self.MainCharacter`)))
  (bind _returnvalue (`SceneComponent.K2_GetComponentLocation` (`MainCharacter.EyesCamera` (`self.MainCharacter`))))
  (bind _location (.location (`SceneComponent.GetSocketTransform` (`Item.ItemMesh` _equippedweapon) "Ironsight" "RTS_World")))
  (bind _returnvalue_2 (- _location _returnvalue))
  (bind _returnvalue_3 (`KismetMathLibrary.GetForwardVector` (.rotation (`SceneComponent.GetSocketTransform` (`Item.ItemMesh` _equippedweapon) "Ironsight" "RTS_World"))))
  (bind _asmain_character (cast `MainCharacter` CameraTarget))
  (bind _output_get (set `self.MainCharacter` _asmain_character))
  (`/Engine/EditorBlueprintResources/StandardMacros.IsValid` _output_get
    (:`Is Valid`
      (if (`ActorComponent.IsActive` (`MainCharacter.EyesCamera` (`self.MainCharacter`)))
        (`/Engine/EditorBlueprintResources/StandardMacros.IsValid` _equippedweapon
          (:`Is Valid`
            (set `self.FinalCameraRotation` (`Pawn.GetControlRotation` (`self.MainCharacter`)))
            (set `self.FinalCameraLocation` (+ (`KismetMathLibrary.VLerp` _returnvalue (- _location (* _returnvalue_3 (* (`KismetMathLibrary.Dot_VectorVector` (`KismetMathLibrary.Normal` _returnvalue_2 0.0) _returnvalue_3) (/ (`KismetMathLibrary.VSize` _returnvalue_2) 250.0)))) (`MainCharacter.CurrentAimValue` (`self.MainCharacter`))) (`KismetMathLibrary.GreaterGreater_VectorRotator` (`self.SwayOffset`) (`self.FinalCameraRotation`))))
            (set `self.FinalCameraFOV` (`KismetMathLibrary.Lerp` 90.0 80.0 (`MainCharacter.CurrentAimValue` (`self.MainCharacter`))))
            (return (`self.FinalCameraLocation`) (`self.FinalCameraRotation`) (`self.FinalCameraFOV`) true)))))))

(fn `UserConstructionScript`)