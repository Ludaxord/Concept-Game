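; Main player character Blueprint that sets up the skill catalog and player UI.
; BeginPlay registers skills in five categories (others are only constructed), then creates HUD, pause, inventory, radial, skill and quest widgets, handing each to its character component and binding quest delegates.
; Inputs toggle inventory, skill and quest screens with input-mode switches, logic marked to move to C++.
; Releasing the held quick-select axis swaps to the weapon chosen in the radial menu.
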(event `self.ReceiveTick`
  (params (DeltaSeconds :type "Float (single-precision)")))

(event `self.ReceiveBeginPlay`
  (`self.InitSkills`)
  (`self.CallBasePlayerHUD`)
  (`self.CallRadialMenu`)
  (`self.CallPauseMenu`)
  (`self.CallSpatialInventoryMenu`)
  (`self.CallSkillsMenu`)
  (`self.CallQuestMenu`)
  (`self.CallQuestInfo`)
  (`self.CallQuestTrackerContainer`)
  (`self.CallQuestUpdatePanel`))

(event `InputAction|Inventory`
  (params (Key :type "Key Structure"))
  (bind _returnvalue (`GameplayStatics.GetPlayerController` 0))
  (bind _returnvalue_2 (`GameplayStatics.GetPlayerController` 0))
  (bind _characterinventorycomponent (`self.CharacterInventoryComponent`))
  (bind _spatialinventorywidget (`InventoryComponent.SpatialInventoryWidget` (`self.CharacterInventoryComponent`)))
  ;[1 1 1] Move To C++
  (:`Pressed`
    (`InventoryComponent.InventoryToggle` _characterinventorycomponent)
    (if (`Widget.IsInViewport` (`InventoryComponent.SpatialInventoryWidget` _characterinventorycomponent))
      (`Widget.RemoveFromParent` (`InventoryComponent.SpatialInventoryWidget` (`self.CharacterInventoryComponent`)))
      (`WidgetBlueprintLibrary.SetInputMode_GameOnly` _returnvalue)
      (set `PlayerController.bShowMouseCursor` false _returnvalue)
      (else
        (`UserWidget.AddToViewport` _spatialinventorywidget 0)
        (`WidgetBlueprintLibrary.SetInputMode_GameAndUIEx` _returnvalue_2 _spatialinventorywidget "DoNotLock" false)
        (set `PlayerController.bShowMouseCursor` true _returnvalue_2)))))

(event `InputAxis|QuickSelect`
  (params (AxisValue :type "Float (single-precision)"))
  (bind _characterinventorycomponent (`self.CharacterInventoryComponent`))
  (bind _quickselectradialmenuwidget (`InventoryComponent.QuickSelectRadialMenuWidget` _characterinventorycomponent))
  (bind _returnvalue (`Widget.IsInViewport` _quickselectradialmenuwidget))
  ;[1 1 1] Move it to C++
  (`InventoryComponent.QuickSelectPieToggle` _characterinventorycomponent (> AxisValue 0.0))
  (if (`InventoryComponent.bQuickSelectVisible` _characterinventorycomponent)
    (if (not _returnvalue)
      (`UserWidget.AddToViewport` _quickselectradialmenuwidget 0)
      (`WidgetBlueprintLibrary.SetInputMode_GameAndUIEx` (`GameplayStatics.GetPlayerController` 0) _quickselectradialmenuwidget "LockAlways" false))
    (elif _returnvalue
      (`Widget.RemoveFromParent` _quickselectradialmenuwidget)
      (bind _asradial_menu_bp (cast `/Game/_Game/HUD/Widgets/RadialMenu/RadialMenuBP` _quickselectradialmenuwidget))
      (`WidgetBlueprintLibrary.SetInputMode_GameOnly` (`GameplayStatics.GetPlayerController` 0))
      (bind _radialmenucirclebp (`/Game/_Game/HUD/Widgets/RadialMenu/RadialMenuBP.RadialMenuCircleBP` _asradial_menu_bp))
      (if (`/Game/_Game/HUD/Widgets/RadialMenu/RadialMenuCircleBP.ItemChanged` _radialmenucirclebp)
        (set `/Game/_Game/HUD/Widgets/RadialMenu/RadialMenuCircleBP.ItemChanged` false _radialmenucirclebp)
        (`InventoryComponent.SwapWeapon` (`self.CharacterInventoryComponent`) (`/Game/_Game/HUD/Widgets/RadialMenu/RadialMenuCircleItemBP.Item` (`/Game/_Game/HUD/Widgets/RadialMenu/RadialMenuCircleBP.Current Item` _radialmenucirclebp)))
        (`KismetSystemLibrary.PrintString` "Item Changed")))))

(event `InputAction|Skills`
  (params (Key :type "Key Structure"))
  (bind _returnvalue (`GameplayStatics.GetPlayerController` 0))
  (bind _characterskillcomponent (`self.CharacterSkillComponent`))
  (bind _skilltreewidget (`SkillComponent.SkillTreeWidget` _characterskillcomponent))
  ;[1 1 1] Move To C++
  (:`Pressed`
    (`SkillComponent.ToggleSkillTree` _characterskillcomponent)
    (if (`Widget.IsInViewport` _skilltreewidget)
      (`Widget.RemoveFromParent` _skilltreewidget)
      (`WidgetBlueprintLibrary.SetInputMode_GameOnly` _returnvalue)
      (set `PlayerController.bShowMouseCursor` false _returnvalue)
      (else
        (`UserWidget.AddToViewport` _skilltreewidget 0)
        (`WidgetBlueprintLibrary.SetInputMode_GameAndUIEx` _returnvalue _skilltreewidget)
        (set `PlayerController.bShowMouseCursor` true _returnvalue)))))

(event `InputAction|Quests`
  (params (Key :type "Key Structure"))
  (bind _returnvalue (`GameplayStatics.GetPlayerController` 0))
  (bind _characterquestsystemcomponent (`self.CharacterQuestSystemComponent`))
  (bind _questlistwidget (`QuestSystemComponent.QuestListWidget` _characterquestsystemcomponent))
  ;[1 1 1] Move To C++
  (:`Pressed`
    (`QuestSystemComponent.QuestListToggle` _characterquestsystemcomponent)
    (if (`Widget.IsInViewport` _questlistwidget)
      (`Widget.RemoveFromParent` _questlistwidget)
      (`WidgetBlueprintLibrary.SetInputMode_GameOnly` _returnvalue)
      (set `PlayerController.bShowMouseCursor` false _returnvalue)
      (else
        (`UserWidget.AddToViewport` _questlistwidget 0)
        (`WidgetBlueprintLibrary.SetInputMode_GameAndUIEx` _returnvalue _questlistwidget)
        (set `PlayerController.bShowMouseCursor` true _returnvalue)))))

(fn `BindOpenQuestInfo`
  (params (bIsClosed :type Boolean) (InQuestName :type String) (InQuestDescription :type String))
  (bind _asquest_info_widget_bp (cast `/Game/_Game/Quests/QuestInfoWidgetBP` (`QuestSystemComponent.QuestInfoWidget` (`self.CharacterQuestSystemComponent`))))
  (`/Game/_Game/Quests/QuestInfoWidgetBP.OpenQuestInfo` _asquest_info_widget_bp bIsClosed InQuestName InQuestDescription))

(fn `CallBasePlayerHUD`
  (bind _characterbasehudcomponent (`self.CharacterBaseHUDComponent`))
  (bind _returnvalue (`|CreateWidget` "/Game/_Game/HUD/Widgets/Game/PlayerHUD.PlayerHUD_C" (`GameplayStatics.GetPlayerController` 0) (`BaseHUDComponent.CurrentMiniMapTexture` _characterbasehudcomponent)))
  (`BaseHUDComponent.CreateBasePlayerHUD` _characterbasehudcomponent _returnvalue))

(fn `CallInventoryMenu`
  (bind _returnvalue (`|CreateWidget` "/Game/_Game/HUD/Widgets/====Inventory--deprecated--/InventoryWidgetBP.InventoryWidgetBP_C" (`GameplayStatics.GetPlayerController` 0)))
  (`InventoryComponent.CreateInventoryWidget` (`self.CharacterInventoryComponent`) _returnvalue (`/Game/_Game/HUD/Widgets/====Inventory--deprecated--/InventoryWidgetBP.InventoryGridBP` _returnvalue) (`/Game/_Game/HUD/Widgets/====Inventory--deprecated--/InventoryWidgetBP.BackgroundBorderBP` _returnvalue)))

(fn `CallPauseMenu`
  (bind _characterpausemenucomponent (`self.CharacterPauseMenuComponent`))
  (bind _returnvalue (`|CreateWidget` "/Game/_Game/HUD/Widgets/Game/PauseMenuWidgetBP.PauseMenuWidgetBP_C" (`GameplayStatics.GetPlayerController` 0)))
  (`/Engine/EditorBlueprintResources/StandardMacros.IsValid` _characterpausemenucomponent
    (:`Is Valid`
      _)
    (:`Is Not Valid`
      (bind _returnvalue_2 (`AddComponent|NODE_AddPauseMenuComponent-0`))
      (set `self.CharacterPauseMenuComponent` _returnvalue_2)))
  (`PauseMenuComponent.CreatePauseMenu` _characterpausemenucomponent _returnvalue))

(fn `CallPostProcess`)

(fn `CallQuestInfo`
  (bind _characterquestsystemcomponent (`self.CharacterQuestSystemComponent`))
  (bind _returnvalue (`|CreateWidget` "/Game/_Game/Quests/QuestInfoWidgetBP.QuestInfoWidgetBP_C" (`GameplayStatics.GetPlayerController` 0) _characterquestsystemcomponent))
  (set `QuestSystemComponent.QuestInfoWidget` _returnvalue _characterquestsystemcomponent)
  (add `QuestSystemComponent.QuestInfoWidgetStateDelegate` _characterquestsystemcomponent (`|CreateDelegate` :!event `BindOpenQuestInfo`)))

(fn `CallQuestMenu`
  (bind _characterquestsystemcomponent (`self.CharacterQuestSystemComponent`))
  (bind _returnvalue (`|CreateWidget` "/Game/_Game/Quests/QuestListWidgetBP.QuestListWidgetBP_C" (`GameplayStatics.GetPlayerController` 0) (`self.CharacterQuestSystemComponent`)))
  (set `QuestSystemComponent.QuestListWidget` _returnvalue _characterquestsystemcomponent)
  (add `QuestSystemComponent.AddRemoveQuestDelegate` _characterquestsystemcomponent (`|CreateDelegate` _returnvalue :!event `UpdateQuestsList`)))

(fn `CallQuestTrackerContainer`
  (bind _characterquestsystemcomponent (`self.CharacterQuestSystemComponent`))
  (bind _returnvalue (`|CreateWidget` "/Game/_Game/Quests/QuestTrackerContainerWidgetBP.QuestTrackerContainerWidgetBP_C" (`GameplayStatics.GetPlayerController` 0) _characterquestsystemcomponent))
  (set `QuestSystemComponent.QuestTrackerContainerWidget` _returnvalue _characterquestsystemcomponent)
  (add `QuestSystemComponent.StepUpdateDelegate` _characterquestsystemcomponent (`|CreateDelegate` _returnvalue :!event `Step Update`)))

(fn `CallQuestUpdatePanel`
  (bind _characterquestsystemcomponent (`self.CharacterQuestSystemComponent`))
  (bind _returnvalue (`|CreateWidget` "/Game/_Game/Quests/QuestUpdatePanelWidgetBP.QuestUpdatePanelWidgetBP_C" (`GameplayStatics.GetPlayerController` 0) _characterquestsystemcomponent))
  (set `QuestSystemComponent.QuestUpdatePanelWidget` _returnvalue _characterquestsystemcomponent)
  (add `QuestSystemComponent.QuestNotificationDelegate` _characterquestsystemcomponent (`|CreateDelegate` _returnvalue :!event `Quest Notification`)))

(fn `CallQuickSelectPieWidget`
  (bind _returnvalue (`|CreateWidget` "/Game/_Game/HUD/Widgets/====PieMenu--deprecated--/PieMenuWidgetBP.PieMenuWidgetBP_C" (`GameplayStatics.GetPlayerController` 0)))
  (`InventoryComponent.CreateQuickSelectPieWidget` (`self.CharacterInventoryComponent`) _returnvalue))

(fn `CallRadialMenu`
  (bind _characterinventorycomponent (`self.CharacterInventoryComponent`))
  (bind _returnvalue (`|CreateWidget` "/Game/_Game/HUD/Widgets/RadialMenu/RadialMenuBP.RadialMenuBP_C" (`GameplayStatics.GetPlayerController` 0) (`InventoryComponent.SectorCount` _characterinventorycomponent) _characterinventorycomponent))
  (set `InventoryComponent.QuickSelectRadialMenuWidget` _returnvalue (`self.CharacterInventoryComponent`)))

(fn `CallSkillsMenu`
  (bind _returnvalue (`|CreateWidget` "/Game/_Game/HUD/Widgets/SkillTree/SkillTreeWidgetBP.SkillTreeWidgetBP_C" (`GameplayStatics.GetPlayerController` 0) (`self.CharacterSkillComponent`)))
  (set `SkillComponent.SkillTreeWidget` _returnvalue (`self.CharacterSkillComponent`)))

(fn `CallSpatialInventoryMenu`
  (bind _returnvalue (`|CreateWidget` "/Game/_Game/HUD/Widgets/Inventory/SpatialInventoryWidgets/SpatialInventoryBP.SpatialInventoryBP_C" (`GameplayStatics.GetPlayerController` 0) (`self.CharacterInventoryComponent`) 50.0))
  (set `InventoryComponent.SpatialInventoryWidget` _returnvalue (`self.CharacterInventoryComponent`)))

(fn `CallTestWidget`
  (bind _returnvalue (`GameplayStatics.GetPlayerController` 0))
  (bind _returnvalue_2 (`GameplayStatics.GetPlayerController` 0))
  (bind _debugwidgetcomponent (`self.DebugWidgetComponent`))
  (set `DebugWidgetComponent.bToggle` (not (`DebugWidgetComponent.bToggle` _debugwidgetcomponent)) _debugwidgetcomponent)
  (if (`DebugWidgetComponent.bToggle` (`self.DebugWidgetComponent`))
    (bind _returnvalue_3 (`|CreateWidget` "/Game/_Game/HUD/Widgets/====TestWidget--deprecated--/TestWidgetBP.TestWidgetBP_C" _returnvalue_2))
    (bind _output_get (set `DebugWidgetComponent.Widget` _returnvalue_3 (`self.DebugWidgetComponent`)))
    (`UserWidget.AddToViewport` _output_get 1)
    (`WidgetBlueprintLibrary.SetInputMode_UIOnlyEx` _returnvalue_2 _returnvalue_3)
    (set `PlayerController.bShowMouseCursor` true _returnvalue_2)
    (else
      (`KismetSystemLibrary.PrintString` "Hello")
      (`WidgetBlueprintLibrary.SetInputMode_GameOnly` _returnvalue)
      (`Widget.RemoveFromParent` (`DebugWidgetComponent.Widget` (`self.DebugWidgetComponent`)))
      (set `PlayerController.bShowMouseCursor` false _returnvalue))))

(fn `InitSkills`
  (`|ExecutionSequence`
    (:`then_0`
      (bind _returnvalue (`|GenericCreateObject` "/Script/Concept_Game.DoubleJumpSkill" self))
      (`DoubleJumpSkill.Init` _returnvalue "Agility" "Double Jump" "Allows to Double Jump" 2 "/Engine/EngineResources/AICON-Green.AICON-Green")
      (bind _returnvalue_2 (`|GenericCreateObject` "/Script/Concept_Game.IncreasedSpeedSkill" self))
      (`IncreasedSpeedSkill.Init` _returnvalue_2 "Agility" "Increased Speed" "Allows to Walk Quicker" 2 "/Engine/EditorResources/Ai_Spawnpoint.Ai_Spawnpoint")
      (`SkillComponent.AddSkills` (`self.CharacterSkillComponent`) "Agility" (`|MakeArray` _returnvalue _returnvalue_2 :!type "Skill Object Reference")))
    (:`then_2`
      (bind _returnvalue_3 (`|GenericCreateObject` "/Script/Concept_Game.AlternativeRoutesHighlightSkill" self))
      (`AlternativeRoutesHighlightSkill.Init` _returnvalue_3 "Map" "" "" 0 null)
      (bind _returnvalue_4 (`|GenericCreateObject` "/Script/Concept_Game.EnemiesMinimapHighlightSkill" self))
      (`EnemiesMinimapHighlightSkill.Init` _returnvalue_4 "Map" "" "" 0 null)
      (bind _returnvalue_5 (`|GenericCreateObject` "/Script/Concept_Game.ItemMinimapHighlightSkill" self))
      (`ItemMinimapHighlightSkill.Init` _returnvalue_5 "Map" "" "" 0 null)
      (bind _returnvalue_6 (`|GenericCreateObject` "/Script/Concept_Game.MiniMapSkill" self))
      (`MiniMapSkill.Init` _returnvalue_6 "Map" "" "" 0 null)
      (`SkillComponent.AddSkills` (`self.CharacterSkillComponent`) "Map" (`|MakeArray` _returnvalue_6 _returnvalue_5 _returnvalue_4 _returnvalue_3 :!type "Skill Object Reference")))
    (:`then_3`
      (bind _returnvalue_7 (`|GenericCreateObject` "/Script/Concept_Game.AreaScanSkill" self))
      (`AreaScanSkill.Init` _returnvalue_7 "Eyes" "" "" 0 null)
      (bind _returnvalue_8 (`|GenericCreateObject` "/Script/Concept_Game.EyeScannerSkill" self))
      (`EyeScannerSkill.Init` _returnvalue_8 "Eyes" "" "" 0 null)
      (`SkillComponent.AddSkills` (`self.CharacterSkillComponent`) "Eyes" (`|MakeArray` _returnvalue_8 _returnvalue_7 :!type "Skill Object Reference")))
    (:`then_4`
      (bind _returnvalue_9 (`|GenericCreateObject` "/Script/Concept_Game.ArmorSkill" self))
      (`ArmorSkill.Init` _returnvalue_9 "Armor" "" "" 0 null)
      (`SkillComponent.AddSkills` (`self.CharacterSkillComponent`) "Armor" (`|MakeArray` _returnvalue_9 :!type "Skill Object Reference")))
    (:`then_5`
      (bind _returnvalue_10 (`|GenericCreateObject` "/Script/Concept_Game.CamoSkill" self))
      (`CamoSkill.Init` _returnvalue_10 "Stealth" "Cloak" "Allows to be invisible" 3 "/Engine/EditorResources/Ai_Spawnpoint.Ai_Spawnpoint")
      (`SkillComponent.AddSkills` (`self.CharacterSkillComponent`) "Stealth" (`|MakeArray` _returnvalue_10 :!type "Skill Object Reference")))
    (:`then_6`
      (`|GenericCreateObject` "/Script/Concept_Game.CarDrivingSkill" self)
      (`|GenericCreateObject` "/Script/Concept_Game.ElectricsTransportSkill" self))
    (:`then_8`
      (`|GenericCreateObject` "/Script/Concept_Game.CombatSkill" self)
      (`|GenericCreateObject` "/Script/Concept_Game.NinjaCombatSkill" self))
    (:`then_9`
      (`|GenericCreateObject` "/Script/Concept_Game.CommunicationSkill" self)
      (`|GenericCreateObject` "/Script/Concept_Game.CommunicationBlockerSkill" self)
      (`|GenericCreateObject` "/Script/Concept_Game.HelicopterFlyingSkill" self))
    (:`then_14`
      (`|GenericCreateObject` "/Script/Concept_Game.HackingSkill" self)
      (`|GenericCreateObject` "/Script/Concept_Game.RemoteHackingSkill" self))
    (:`then_15`
      (`|GenericCreateObject` "/Script/Concept_Game.HandBladesSkill" self)
      (`|GenericCreateObject` "/Script/Concept_Game.HandBladesWallMovingSkill" self))
    (:`then_17`
      (`|GenericCreateObject` "/Script/Concept_Game.HeavyItemMovementSkill" self)
      (`|GenericCreateObject` "/Script/Concept_Game.ItemMovementSkill" self))
    (:`then_19`
      (`|GenericCreateObject` "/Script/Concept_Game.InventorySizeX2Skill" self)
      (`|GenericCreateObject` "/Script/Concept_Game.InventorySizeX4Skill" self)
      (`|GenericCreateObject` "/Script/Concept_Game.InventorySkill" self)
      (`|GenericCreateObject` "/Script/Concept_Game.QuickSelectSkill" self))
    (:`then_24`
      (`|GenericCreateObject` "/Script/Concept_Game.LungsEnhacementSkill" self))
    (:`then_25`
      (`|GenericCreateObject` "/Script/Concept_Game.MarksmanSkill" self))
    (:`then_28`
      (`|GenericCreateObject` "/Script/Concept_Game.ParkourFloorSlideSkill" self)
      (`|GenericCreateObject` "/Script/Concept_Game.ParkourWallRunningSkill" self))
    (:`then_36`
      (`|GenericCreateObject` "/Script/Concept_Game.SwimmingSkill" self))))

(fn `UserConstructionScript`)